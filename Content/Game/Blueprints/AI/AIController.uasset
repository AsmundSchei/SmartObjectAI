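; AI controller that starts a behavior tree and feeds perception results into its blackboard, treating player 0 as the enemy.
; Perception updates set whether the player is seen and store their current location when sight is lost.
; Target perception updates set or clear FindPlayer for any sensed actor, flagging investigation at the stimulus location on success.
; A random-roam loop and debug sphere are left unconnected.
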(event `self.ReceiveBeginPlay`
  (bind _returnvalue (`GameplayStatics.GetPlayerCharacter` 0))
  (`|ExecutionSequence`
    (:`then_1`
      (`self.UseBlackboard` "/Game/Game/Blueprints/AI/AIBlackboard.AIBlackboard")
      (`self.RunBehaviorTree` "/Game/Game/Blueprints/AI/AIBehaviourTree.AIBehaviourTree")
      (set `self.Enemy` _returnvalue)
      (`BlackboardComponent.SetValueAsObject` (`self.Blackboard`) "Enemy" _returnvalue))))

(event `self.AIPerception.OnPerceptionUpdated`
  (params (UpdatedActors :type "Array of Actor Object Reference (by ref)"))
  (bind _returnvalue (`AIBlueprintHelperLibrary.GetBlackboard` null))
  (for _array_element UpdatedActors
    (if (== _array_element (`self.Enemy`))
      (bind _info (`AIPerceptionComponent.GetActorsPerception` (`self.AIPerception`) _array_element))
      (bind (_age _expirationage _strength _stimuluslocation _receiverlocation _tag _bsuccessfullysensed) (break `AIStimulus` (`|GetArrayItem` (`.LastSensedStimuli` (break `ActorPerceptionBlueprintInfo` _info)))))
      (`BlackboardComponent.SetValueAsBool` _returnvalue "CanSeePlayer" _bsuccessfullysensed)
      (if (not _bsuccessfullysensed)
        (`BlackboardComponent.SetValueAsVector` _returnvalue "LastSeenLocation" (`self.K2_GetActorLocation` (`self.Enemy`)))))))

(event `self.AIPerception.OnTargetPerceptionUpdated`
  (params (Actor :type "Actor Object Reference") (Stimulus :type "AIStimulus Structure"))
  (bind (_age _expirationage _strength _stimuluslocation _receiverlocation _tag _bsuccessfullysensed) (break `AIStimulus` Stimulus))
  (if (`.bSuccessfullySensed` (break `AIStimulus` Stimulus))
    (`BlackboardComponent.SetValueAsObject` (`self.Blackboard`) "FindPlayer" Actor)
    (bind _returnvalue (`AIPerceptionSystem.GetSenseClassForStimulus` Stimulus))
    (switch `string` (`KismetSystemLibrary.GetClassDisplayName` _returnvalue)
      (:`Default`
        (`BlackboardComponent.SetValueAsBool` (`self.Blackboard`) "Investigate" _bsuccessfullysensed)
        (if _bsuccessfullysensed
          (`BlackboardComponent.SetValueAsVector` (`self.Blackboard`) "TargetLocation" _stimuluslocation))))
    (else
      (`BlackboardComponent.SetValueAsObject` (`self.Blackboard`) "FindPlayer" null))))

(fn `UserConstructionScript`)