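; AI gun actor with a weapon-switch animation and an optional laser sight.
; Appear and Dissapear play the SwitchWeapon timeline forward or backward to offset GunMesh's relative location, with Dissapear also flagging SwitchingWeapons.
; SpawnLaserParticle attaches a beam emitter at LaserStart and sets its endpoint using a visibility trace along the Arrow's forward vector.
; BeginPlay is empty, and the startup calls to Appear and the laser timer are disconnected.
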(event `Appear`
  ;[0 0.2438 0.7083] Pulls up/down weapon during weapon switching (Dont change/delete this!)
  (bind (_direction _switchweapon) (`Timeline|SwitchWeapon` :!via `PlayFromStart` :!label _label)
    (:`Update`
      _)
    (:`Finished`
      _))
  (`SceneComponent.K2_SetRelativeLocation` (`self.GunMesh`) (`KismetMathLibrary.Conv_DoubleToVector` (* _switchweapon -1.0)) false false))

(event `Dissapear`
  ;[0 0.2438 0.7083] Pulls up/down weapon during weapon switching (Dont change/delete this!)
  (set `self.SwitchingWeapons` true)
  (goto _label :!via `ReverseFromEnd`))

(event `self.ReceiveBeginPlay`)

(fn `SpawnLaserParticle`
  (bind _returnvalue (`SceneComponent.K2_GetComponentLocation` (`self.LaserStart`)))
  (`GameplayStatics.SpawnEmitterAttached` (`self.LaserParticle`) (`self.LaserStart`))
  (`/Engine/EditorBlueprintResources/StandardMacros.IsValid` null
    (:`Is Valid`
      (`ParticleSystemComponent.SetBeamSourcePoint` (`self.LaserSourcePoint`) 0 _returnvalue 0)
      (`ParticleSystemComponent.SetBeamTargetPoint` (`self.LaserSourcePoint`) 0 (0.0 0.0 0.0) 0)
      (bind (_outhit _returnvalue_2) (`KismetSystemLibrary.LineTraceSingle` _returnvalue (+ _returnvalue (* (`SceneComponent.GetForwardVector` (`self.Arrow`)) 2000.0)) "TraceTypeQuery1"))
      (if _returnvalue_2
        (bind (_bblockinghit _binitialoverlap _time _distance _location _impactpoint _normal _impactnormal _physmat _hitactor _hitcomponent _hitbonename _bonename _hititem _elementindex _faceindex _tracestart _traceend) (`GameplayStatics.BreakHitResult` _outhit))
        (`ParticleSystemComponent.SetBeamTargetPoint` (`self.LaserSourcePoint`) 0 (`KismetMathLibrary.SelectVector` _location _traceend _bblockinghit) 0)))))

(fn `UserConstructionScript`)